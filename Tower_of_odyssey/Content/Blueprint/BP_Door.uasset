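; BP_Door is an interactable door that swings open and closed.
; Interact flips a Status between Closed and Open, playing or reversing the DoorMechanic timeline, whose DoorZRotation track sets the yaw of the SMDoor mesh's relative rotation.
; ShowInfo writes a state-dependent "Press [E]" prompt to the HUD it receives.
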(event `/Game/Blueprint/I_Interactable.Interact`
  (switch `/Game/Blueprint/EN_doorStatus` (`self.Status`)
    (:`NewEnumerator0`
      (set `self.Status` "NewEnumerator1")
      (bind (_direction _door_z_rotation) (`Timeline|DoorMechanic` :!label _label)
        (:`Update`
          (`SceneComponent.K2_SetRelativeRotation` (`self.SM_Door`) (`KismetMathLibrary.MakeRotator` 0.0 0.0 _door_z_rotation) false false))))
    (:`NewEnumerator1`
      (set `self.Status` "NewEnumerator0")
      (goto _label :!via `Reverse`))))

(event `/Game/Blueprint/I_Interactable.Show Info`
  (params (HUD :type "/Game/Widgit/WBP_HUD Object Reference"))
  (switch `/Game/Blueprint/EN_doorStatus` (`self.Status`)
    (:`NewEnumerator0`
      (`/Game/Widgit/WBP_HUD.SetInfoText` HUD "Press [E] to Open Door"))
    (:`NewEnumerator1`
      (`/Game/Widgit/WBP_HUD.SetInfoText` HUD "Press [E] to Close Door"))))

(fn `UserConstructionScript`)