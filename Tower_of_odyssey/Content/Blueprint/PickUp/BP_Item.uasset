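; BP_Item is a pickup actor whose static mesh is set from ItemModelToPlace in the construction script.
; ShowInfo puts an "[E] to PickUp" prompt on the supplied HUD.
; Pickable plays a timeline that scales the root down to zero.
; A DoOnce on the timeline's first update plays the pickup sound, then destroys the actor after a short fixed delay, independent of the timeline finishing.
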(event `/Game/Blueprint/BPI_Interactable.Pickable`
  (`KismetSystemLibrary.PrintString` "Item Picked")
  (bind (_direction _shrinktimeline) (`Timeline|Shrink`)
    (:`Update`
      (`SceneComponent.SetWorldScale3D` (`self.DefaultSceneRoot`) (`KismetMathLibrary.Conv_DoubleToVector` (`KismetMathLibrary.Lerp` 1.0 0.0 _shrinktimeline)))
      (`/Engine/EditorBlueprintResources/StandardMacros.DoOnce` false
        (:`Completed`
          (`GameplayStatics.PlaySound2D` "/Engine/VREditor/Sounds/UI/Object_PickUp.Object_PickUp" 1.0 1.0 0.0 null null)
          (`KismetSystemLibrary.Delay` 0.4)
          (`self.K2_DestroyActor`))))))

(event `/Game/Blueprint/BPI_Interactable.Show Info`
  (params (HUD :type "/Game/HUD/main/WBP_HUD Object Reference"))
  (`/Game/HUD/main/WBP_HUD.SetInfoText` HUD "Press [E] to PickUp"))

(fn `UserConstructionScript`
  (`StaticMeshComponent.SetStaticMesh` (`self.SM_ItemModel`) (`self.ItemModelToPlace`)))